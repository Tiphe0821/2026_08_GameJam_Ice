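; BP_Objective is the goal object in IceEscape that ends play with a finish screen when it registers a Hit.
; The first Hit sets the IsFinish flag, adds WBP_FinishUI to the viewport, shows the mouse cursor and switches player 0 to UI-only input.
; Completion relies on physical hits rather than overlap, with no check on the hitting actor, and the debug "Finish!" message prints on every hit.
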(event EventBeginPlay
  (Variables|Default|SetIsFinish false))

(event Collision|EventActorBeginOverlap
  (params (OtherActor :type Actor%20Object%20Reference)))

(event EventTick
  (params (DeltaSeconds :type Float%20%28single-precision%29)))

(event Collision|EventHit
  (params (MyComp :type Primitive%20Component%20Object%20Reference) (Other :type Actor%20Object%20Reference) (OtherComp :type Primitive%20Component%20Object%20Reference) (bSelfMoved :type Boolean) (HitLocation :type Vector :default "0, 0, 0") (HitNormal :type Vector :default "0, 0, 0") (NormalImpulse :type Vector :default "0, 0, 0") (Hit :type Hit%20Result%20Structure%20%28by%20ref%29))
  (bind _returnvalue (Game|GetPlayerController 0))
  (Development|PrintString "Finish!")
  (if (not (Variables|Default|GetIsFinish))
    (Variables|Default|SetIsFinish true)
    (bind _returnvalue_2 (UserInterface|CreateWidget "/Game/IceEscape/UI/WBP_FinishUI.WBP_FinishUI_C" (Game|GetPlayerController 0)))
    (UserInterface|Viewport|AddtoViewport _returnvalue_2 0)
    (Variables|/Script/Engine.PlayerController|SetbShowMouseCursor _returnvalue true)
    (Input|SetInputModeUIOnly _returnvalue 0 "DoNotLock" false)))

(fn ConstructionScript)